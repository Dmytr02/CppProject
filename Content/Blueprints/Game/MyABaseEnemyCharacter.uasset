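; Base enemy character Blueprint that displays a health bar through a widget component.
; On BeginPlay it binds to the health-changed event, whose handler makes the WBP_Healse progress bar fully opaque and sets its fill to new health over MaxHealth.
; Every Tick it rotates the widget component to face the player camera, billboarding the bar in world space.
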(event `self.ReceiveBeginPlay`
  (add `self.OnHealseChanged` (delegate `CustomEvent`)))

(event `CustomEvent` :!signature `self.OnHealseChanged`
  (params (NewHealse :type Integer))
  (bind _aswbp_healse (cast `/Game/Blueprints/UI/WBP_Healse` (`WidgetComponent.GetWidget` (`self.Widget`))))
  (bind _progressbar_45 (`/Game/Blueprints/UI/WBP_Healse.ProgressBar_45` _aswbp_healse))
  (`Widget.SetRenderOpacity` _progressbar_45 1.0)
  (`ProgressBar.SetPercent` _progressbar_45 (/ (`KismetMathLibrary.Conv_IntToDouble` NewHealse) (`KismetMathLibrary.Conv_IntToDouble` (`self.MaxHealth`)))))

(event `self.ReceiveTick`
  (params (DeltaSeconds :type "Float (single-precision)"))
  (bind _widget (`self.Widget`))
  (`SceneComponent.K2_SetWorldRotation` _widget (`KismetMathLibrary.FindLookAtRotation` (`SceneComponent.K2_GetComponentLocation` _widget) (`PlayerCameraManager.GetCameraLocation` (`GameplayStatics.GetPlayerCameraManager` 0))) false false))

(fn `UserConstructionScript`)