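; Player character Blueprint that creates the main HUD on BeginPlay and keeps it in sync with health, stamina and character state.
; Both progress bars start full, then update as current-to-max ratios through events bound to the health and stamina change notifications.
; The character state text is not event-driven: Tick rewrites it from the state enum's name every frame.
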(event `self.ReceiveBeginPlay`
  (add `self.OnStaminaChanged` (delegate `OnStaminaChanged_Event`))
  (add `self.OnHealseChanged` (delegate `OnHealseChanged_Event`))
  (bind _returnvalue (`|CreateWidget` "/Game/Blueprints/UI/WBP_MainHUD.WBP_MainHUD_C"))
  (`UserWidget.AddToViewport` _returnvalue 0)
  (`ProgressBar.SetPercent` (`/Game/Blueprints/UI/WBP_MainHUD.ProgressBar_61` _returnvalue) 1.0)
  (`ProgressBar.SetPercent` (`/Game/Blueprints/UI/WBP_MainHUD.ProgressBar` _returnvalue) 1.0))

(event `OnHealseChanged_Event` :!signature `self.OnHealseChanged`
  (params (NewHealse :type Integer))
  (`ProgressBar.SetPercent` (`/Game/Blueprints/UI/WBP_MainHUD.ProgressBar_61` (stale `self.ReceiveBeginPlay` _returnvalue)) (/ (`KismetMathLibrary.Conv_IntToDouble` NewHealse) (`KismetMathLibrary.Conv_IntToDouble` (`self.MaxHealth`)))))

(event `OnStaminaChanged_Event` :!signature `self.OnStaminaChanged`
  (params (NewStamina :type "Float (single-precision)"))
  (`ProgressBar.SetPercent` (`/Game/Blueprints/UI/WBP_MainHUD.ProgressBar` (stale `self.ReceiveBeginPlay` _returnvalue)) (/ NewStamina (`self.MaxStamina`))))

(event `self.ReceiveTick`
  (params (DeltaSeconds :type "Float (single-precision)"))
  (set `TextBlock.Text` (`KismetTextLibrary.Conv_StringToText` (`|GetEnumeratorNameAsString` (`self.CharacterState`))) (`/Game/Blueprints/UI/WBP_MainHUD.TextBlock_0` (stale `self.ReceiveBeginPlay` _returnvalue))))

(fn `UserConstructionScript`)